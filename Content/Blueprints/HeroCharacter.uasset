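; Player hero character for a twin-stick shooter, handling movement, aiming, firing and death.
; On BeginPlay it spawns and attaches a weapon to GunT and records its transform as the TwinStickGameMode respawn point.
; Move axes drive world-space movement, while both look axes share one branch that sets control rotation and holds the trigger beyond a deadzone.
; AffectHealth recalculates health and, on death, requests a respawn and destroys hero and weapon.
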(event EventBeginPlay
  (bind _gunt (Variables|Default|GetGunT))
  (Utilities|FlowControl|Sequence
    (:then_0
      (bind _returnvalue (Game|SpawnActorfromClass "/Game/Blueprints/Weapon.Weapon_C" (Transformation|GetWorldTransform _gunt) "Undefined" 0 0))
      (bind _output_get (Variables|Default|SetWeapon _returnvalue))
      (Transformation|AttachComponentToComponent _output_get _gunt "None" "SnapToTarget" "KeepRelative" "KeepRelative" true))
    (:then_1
      (bind _astwin_stick_game_mode (Utilities|Casting|CastToTwinStickGameMode (Game|GetGameMode)))
      (bind _output_get_2 (Variables|Default|SetGameMode _astwin_stick_game_mode))
      (Variables|/Game/Blueprints/TwinStickGameMode.TwinStickGameMode_C|SetPlayerSpawnTransform _output_get_2 (Transformation|GetActorTransform)))))

(event EventAffectHealth
  (params (Delta :type Float%20%28single-precision%29))
  (Class|BaseCharacter|CalculateHealth Delta)
  (if (Variables|Default|GetisDead)
    (Default|RespawnHero (Variables|Default|GetGameMode))
    (Actor|DestroyActor (Variables|Default|GetWeapon))))

(event Input|AxisEvents|InputAxisMoveUp
  (params (AxisValue :type Float%20%28single-precision%29))
  ;[1 1 1] Moment
  (Pawn|Input|AddMovementInput "1.000000, 0, 0" AxisValue false))

(event Input|AxisEvents|InputAxisMoveRight
  (params (AxisValue :type Float%20%28single-precision%29))
  ;[1 1 1] Moment
  (Pawn|Input|AddMovementInput "0.000000,1.000000, 0" AxisValue false))

(event Input|AxisEvents|InputAxisLookUp
  (params (AxisValue :type Float%20%28single-precision%29))
  (bind _weapon (Variables|Default|GetWeapon))
  ;[1 1 1] Rotation
  (if (> (Math|Vector|VectorLength (Math|Vector|MakeVector AxisValue (stale Input|AxisEvents|InputAxisLookRight AxisValue) 0.0)) 0.5)
    (Pawn|SetControlRotation (Pawn|GetController) (Math|Conversions|RotationFromXVector (Math|Vector|MakeVector AxisValue (stale Input|AxisEvents|InputAxisLookRight AxisValue) 0.0)))
    (Default|PullTrigger _weapon)
    (else
      (Default|ReleaseTrigger _weapon))))

(event Input|AxisEvents|InputAxisLookRight
  (params (AxisValue :type Float%20%28single-precision%29))
  (bind _weapon (Variables|Default|GetWeapon))
  ;[1 1 1] Rotation
  (if (> (Math|Vector|VectorLength (Math|Vector|MakeVector (stale Input|AxisEvents|InputAxisLookUp AxisValue) AxisValue 0.0)) 0.5)
    (Pawn|SetControlRotation (Pawn|GetController) (Math|Conversions|RotationFromXVector (Math|Vector|MakeVector (stale Input|AxisEvents|InputAxisLookUp AxisValue) AxisValue 0.0)))
    (Default|PullTrigger _weapon)
    (else
      (Default|ReleaseTrigger _weapon))))

(fn ConstructionScript)