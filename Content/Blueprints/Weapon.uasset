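; Weapon Blueprint that fires projectiles automatically while its trigger is held.
; PullTrigger passes a DoOnce gate, fires immediately, then starts a looping timer on Fire at an interval derived from FirePerSec.
; ReleaseTrigger clears the timer and resets the gate, so repeated pulls cannot restart firing until release.
; Each Fire spawns the Projectile class at the Arrow component's world transform.
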(event Custom|Pull%20Trigger
  (Utilities|FlowControl|DoOnce false
    (:Completed
      (CallFunction|Fire)
      (Utilities|Time|SetTimerbyFunctionName 0 "Fire" (/ 1.0 (Variables|Default|GetFirePerSec)) true))))

(event Custom|Fire
  (Game|SpawnActorfromClass "/Game/Blueprints/Projectile.Projectile_C" (Transformation|GetWorldTransform (Variables|Default|GetArrow)) "Undefined" 0 0))

(event Custom|ReleaseTrigger
  (Utilities|Time|ClearTimerbyFunctionName 0 "Fire")
  (Utilities|FlowControl|DoOnce false) ; enters at Reset
)

(fn ConstructionScript)